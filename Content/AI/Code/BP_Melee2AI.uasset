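; BP_Melee2AI is a melee enemy that spots the player and reports its state to MyGameState.
; It caches the player character and game state on BeginPlay.
; When PawnSensing sees the player, ChasePlayer sets the SeenPlayer blackboard key, prints a debug string and notifies the game state.
; A hit against the player calls the game state's enemy death notification, with no damage or destroy logic here.
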(event OnSeePawn(PawnSensing)
  (params (Pawn :type Pawn%20Object%20Reference))
  (if (== Pawn (Variables|Default|GetPlayer))
    (CallFunction|ChasePlayer)))

(event EventBeginPlay
  (Variables|Default|SetPlayer (Game|GetPlayerCharacter 0))
  (bind _asmy_game_state (Utilities|Casting|CastToMyGameState (Game|GetGameState)))
  (Variables|Default|SetAs%20My%20Game%20State _asmy_game_state))

(event Collision|EventHit
  (params (MyComp :type Primitive%20Component%20Object%20Reference) (Other :type Actor%20Object%20Reference) (OtherComp :type Primitive%20Component%20Object%20Reference) (bSelfMoved :type Boolean) (HitLocation :type Vector :default "0, 0, 0") (HitNormal :type Vector :default "0, 0, 0") (NormalImpulse :type Vector :default "0, 0, 0") (Hit :type Hit%20Result%20Structure%20%28by%20ref%29))
  (if (== Other (Variables|Default|GetPlayer))
    (Default|CallOnEnemyDeath (Variables|Default|GetAs%20My%20Game%20State) self)))

(fn ConstructionScript)

(fn ChasePlayer
  (AI|Components|Blackboard|SetValueasBool (AI|GetBlackboard (AI|GetAIController self)) (Utilities|Name|MakeLiteralName "SeenPlayer") true)
  (Development|PrintString "should chase player")
  (Default|CallOnSeenPlayer (Variables|Default|GetAs%20My%20Game%20State) self))